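; BP_Ladder is a ladder actor that tells BP_Player when it is near a ladder and where its key points are.
; Overlapping the bottom trigger flags the player as near and passes the lower lock transform plus upper and lower borders.
; The top trigger also flags a possible ladder exit, passing the upper lock and finish spawn transforms, but no borders.
; Leaving either trigger clears its flags; the ladder itself contains no movement logic.
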(event `self.DownEnterTrigger.OnComponentBeginOverlap`
  (params (OverlappedComponent :type "PrimitiveComponent Object Reference") (OtherActor :type "Actor Object Reference") (OtherComp :type "PrimitiveComponent Object Reference") (OtherBodyIndex :type Integer) (bFromSweep :type Boolean) (SweepResult :type "HitResult Structure (by ref)"))
  (bind _returnvalue (`SceneComponent.K2_GetComponentToWorld` (`self.DownLockPoint`)))
  (bind _asbp_player (cast `/Game/ThirdPerson/Blueprints/BP_Player` OtherActor))
  (set `/Game/ThirdPerson/Blueprints/BP_Player.IsNearLadder` true _asbp_player)
  (set `/Game/ThirdPerson/Blueprints/BP_Player.LadderLock` _returnvalue _asbp_player)
  (set `/Game/ThirdPerson/Blueprints/BP_Player.UpBorder` (`SceneComponent.K2_GetComponentToWorld` (`self.UpperLockPoint`)) _asbp_player)
  (set `/Game/ThirdPerson/Blueprints/BP_Player.DownBorder` _returnvalue _asbp_player))

(event `self.DownEnterTrigger.OnComponentEndOverlap`
  (params (OverlappedComponent :type "PrimitiveComponent Object Reference") (OtherActor :type "Actor Object Reference") (OtherComp :type "PrimitiveComponent Object Reference") (OtherBodyIndex :type Integer))
  (bind _asbp_player (cast `/Game/ThirdPerson/Blueprints/BP_Player` OtherActor))
  (set `/Game/ThirdPerson/Blueprints/BP_Player.IsNearLadder` false _asbp_player))

(event `self.UpperEnterTrigger.OnComponentBeginOverlap`
  (params (OverlappedComponent :type "PrimitiveComponent Object Reference") (OtherActor :type "Actor Object Reference") (OtherComp :type "PrimitiveComponent Object Reference") (OtherBodyIndex :type Integer) (bFromSweep :type Boolean) (SweepResult :type "HitResult Structure (by ref)"))
  (bind _asbp_player (cast `/Game/ThirdPerson/Blueprints/BP_Player` OtherActor))
  (set `/Game/ThirdPerson/Blueprints/BP_Player.IsNearLadderOut` true _asbp_player)
  (set `/Game/ThirdPerson/Blueprints/BP_Player.LadderOut` (`SceneComponent.K2_GetComponentToWorld` (`self.FinishSpawnPoint`)) _asbp_player)
  (set `/Game/ThirdPerson/Blueprints/BP_Player.LadderLock` (`SceneComponent.K2_GetComponentToWorld` (`self.UpperLockPoint`)) _asbp_player)
  (set `/Game/ThirdPerson/Blueprints/BP_Player.IsNearLadder` true _asbp_player))

(event `self.UpperEnterTrigger.OnComponentEndOverlap`
  (params (OverlappedComponent :type "PrimitiveComponent Object Reference") (OtherActor :type "Actor Object Reference") (OtherComp :type "PrimitiveComponent Object Reference") (OtherBodyIndex :type Integer))
  (bind _asbp_player (cast `/Game/ThirdPerson/Blueprints/BP_Player` OtherActor))
  (set `/Game/ThirdPerson/Blueprints/BP_Player.IsNearLadderOut` false _asbp_player)
  (set `/Game/ThirdPerson/Blueprints/BP_Player.IsNearLadder` false _asbp_player))

(fn `UserConstructionScript`)